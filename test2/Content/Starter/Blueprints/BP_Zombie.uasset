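; BP_Zombie is an enemy character that chases the player on sight and dies when its Life runs out.
; Pawn sensing sets a seen flag and calls the follow event, which runs AI MoveTo targeting the player controller rather than its pawn.
; Tick polls Life, which starts at three and is not decremented here; at zero, a DoOnce plays the death animation, disables movement and destroys the actor after a delay.
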(event OnSeePawn(PawnSensing)
  (params (Pawn :type Pawn%20Object%20Reference))
  (Variables|Default|Setseeplayer? true)
  (CallFunction|Folloplayer))

(event Custom|folloplayer
  (if (Variables|Default|Getseeplayer?)
    (AI|AIMoveTo self "0, 0, 0" (Game|GetPlayerController 0) 5.0 false)))

(event EventBeginPlay
  (Variables|Default|Setlife 3))

(event Collision|EventActorBeginOverlap
  (params (OtherActor :type Actor%20Object%20Reference)))

(event EventTick
  (params (DeltaSeconds :type Float%20%28single-precision%29))
  (if (== (Variables|Default|Getlife) 0)
    (Utilities|FlowControl|DoOnce false
      (:Completed
        (Components|Animation|PlayAnimation (Variables|Character|GetMesh) "/Game/Starter/Assets/Zombie/Animations/Zombie_Death.Zombie_Death" false)
        (Pawn|Components|CharacterMovement|DisableMovement (Variables|Character|GetCharacterMovement))
        (Utilities|FlowControl|Delay 3.0)
        (Actor|DestroyActor)))))

(fn ConstructionScript)