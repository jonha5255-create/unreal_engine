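; Granny is a playable third-person character with Enhanced Input movement, jumping, Shift sprint and gun combat against zombies.
; Right mouse aims when a gun is held, switching to a close over-the-shoulder camera and controller-driven rotation.
; While aiming, left mouse plays the fire montage and line-traces from the muzzle, spawning an explosion on hits and decrementing BP_Zombie life.
; Tick updates horizontal speed and also runs the muzzle trace while aiming, without using its result.
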(event Input|EnhancedActionEvents|EnhancedInputActionIA_MoveGranny
  (params (ActionValue :type Vector%202D%20Structure) (ElapsedSeconds :type Float%20%28double-precision%29) (TriggeredSeconds :type Float%20%28double-precision%29) (InputAction :type Input%20Action%20Object%20Reference :default "/Game/Starter/Assets/Inputs/IA_MoveGranny.IA_MoveGranny"))
  (bind _returnvalue (Pawn|GetControlRotation :!class /Script/Engine.Pawn))
  ;[0.15 0.15 0.15 0.5] RPG Style
  (Pawn|Input|AddMovementInput (Math|Vector|GetForwardVector (Math|Rotator|MakeRotator 0.0 0.0 (.yaw _returnvalue))) (.x ActionValue) false)
  (Pawn|Input|AddMovementInput (Math|Vector|GetRightVector (Math|Rotator|MakeRotator 0.0 0.0 (.yaw _returnvalue))) (.y ActionValue) false))

(event Input|EnhancedActionEvents|EnhancedInputActionIA_JumpGranny
  (params (ActionValue :type Boolean) (ElapsedSeconds :type Float%20%28double-precision%29) (TriggeredSeconds :type Float%20%28double-precision%29) (InputAction :type Input%20Action%20Object%20Reference :default "/Game/Starter/Assets/Inputs/IA_JumpGranny.IA_JumpGranny"))
  (:Started
    (Character|Jump)))

(event EventBeginPlay)

(event Collision|EventActorBeginOverlap
  (params (OtherActor :type Actor%20Object%20Reference)))

(event EventTick
  (params (DeltaSeconds :type Float%20%28single-precision%29))
  (Variables|Default|SetSpeed (Math|Vector|VectorLengthXY (Transformation|GetVelocity)))
  (if (Variables|Default|GetAIm?)
    (CallFunction|Firemuzzle)))

(event Input|KeyboardEvents|LeftShift
  (params (Key :type Key%20Structure :default "None"))
  (bind _charactermovement (Variables|Character|GetCharacterMovement))
  (:Pressed
    (Variables|/Script/Engine.CharacterMovementComponent|SetMaxWalkSpeed _charactermovement 852.0))
  (:Released
    (Variables|/Script/Engine.CharacterMovementComponent|SetMaxWalkSpeed _charactermovement 426.0)))

(event Input|MouseEvents|LeftMouseButton
  (params (Key :type Key%20Structure :default "None"))
  (:Pressed
    (if (Variables|Default|GetAIm?)
      (Animation|Montage|PlayMontage (Variables|Character|GetMesh) "/Game/Starter/Blueprints/GrannyMontage.GrannyMontage" 1.0 0.0 "fire"
        (:then
          (bind (_hit_ _result) (CallFunction|Firemuzzle))
          (if _hit_
            (Effects|SpawnEmitteratLocation "/Game/StarterContent/Particles/P_Explosion.P_Explosion" (.location _result) "0, 0, 0" "0.300000,0.300000,0.300000")
            (bind _asbp_zombie (Utilities|Casting|CastToBP_Zombie (.hitactor _result)))
            (Math|Integer|DecrementInt (Variables|/Game/Starter/Blueprints/BP_Zombie.BP_Zombie_C|Getlife _asbp_zombie))))))))

(event Input|MouseEvents|RightMouseButton
  (params (Key :type Key%20Structure :default "None"))
  (bind _charactermovement (Variables|Character|GetCharacterMovement))
  (:Pressed
    (if (Variables|Default|GetHaveGun?)
      (Variables|Default|SetAIm? true)
      (Variables|/Script/Engine.SpringArmComponent|SetTargetArmLength (Variables|Default|GetSpringArm) 1.5e+02)
      (Transformation|SetRelativeLocation (Variables|Default|GetCamera) "0.000000,100.000000,50.000000" false false)
      (Variables|Default|SetbUseControllerRotationYaw true)
      (Variables|/Script/Engine.CharacterMovementComponent|SetbOrientRotationToMovement _charactermovement false)
      (Animation|Montage|PlayMontage (Variables|Character|GetMesh) "/Game/Starter/Blueprints/GrannyMontage.GrannyMontage" 1.0 0.0 "Aim")))
  (:Released
    (Variables|Default|SetAIm? false)
    (Variables|/Script/Engine.SpringArmComponent|SetTargetArmLength (Variables|Default|GetSpringArm) 3e+02)
    (Transformation|SetRelativeLocation (Variables|Default|GetCamera) "0.000000,0.000000,0.000000" false false)
    (Variables|Default|SetbUseControllerRotationYaw false)
    (Variables|/Script/Engine.CharacterMovementComponent|SetbOrientRotationToMovement _charactermovement true)
    (Animation|StopAnimMontage "/Game/Starter/Blueprints/GrannyMontage.GrannyMontage")))

(fn ConstructionScript)

(fn Firemuzzle
  (bind _muzzle (Variables|Default|Getmuzzle))
  (bind _returnvalue (Transformation|GetWorldLocation _muzzle))
  (bind (_outhit _returnvalue_2) (Collision|LineTraceByChannel _returnvalue (+ _returnvalue (* (Math|Vector|GetForwardVector _muzzle) 1e+04)) "TraceTypeQuery1" false 0 "None"))
  (return _returnvalue_2 _outhit))