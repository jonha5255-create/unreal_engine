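; Player controller that switches the player from an aircraft to a Granny pawn and handles her death near the ground.
; Space, while Transform is set, replaces and possesses the pawn and swaps Enhanced Input contexts; shared rotate actions drive yaw and pitch.
; A later press below a height threshold clears the Down flag.
; Tick checks height, and if Down remains set, plays a death animation once, then reloads StarterMap after a delay.
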(event Input|EnhancedActionEvents|EnhancedInputActionIA_RotateGranny
  (params (ActionValue :type Vector%202D%20Structure) (ElapsedSeconds :type Float%20%28double-precision%29) (TriggeredSeconds :type Float%20%28double-precision%29) (InputAction :type Input%20Action%20Object%20Reference :default "/Game/Starter/Assets/Inputs/IA_RotateGranny.IA_RotateGranny"))
  (Class|PlayerController|AddYawInput (.x ActionValue))
  (Class|PlayerController|AddPitchInput (.y ActionValue)))

(event Input|EnhancedActionEvents|EnhancedInputActionIA_RotateAircraft
  (params (ActionValue :type Vector%202D%20Structure) (ElapsedSeconds :type Float%20%28double-precision%29) (TriggeredSeconds :type Float%20%28double-precision%29) (InputAction :type Input%20Action%20Object%20Reference :default "/Game/Starter/Assets/Inputs/IA_RotateAircraft.IA_RotateAircraft"))
  (Class|PlayerController|AddYawInput (.x ActionValue))
  (Class|PlayerController|AddPitchInput (.y ActionValue)))

(event EventBeginPlay
  (Input|AddMappingContext (PlayerController|LocalPlayerSubsystems|GetEnhancedInputLocalPlayerSubsystem) "/Game/Starter/Assets/Inputs/IMC_AircraftControl.IMC_AircraftControl" 0 "(bIgnoreAllPressedKeysUntilRelease=True,bForceImmediately=False,bNotifyUserSettings=False)"))

(event EventTick
  (params (DeltaSeconds :type Float%20%28single-precision%29))
  (bind _returnvalue (Game|Player|GetPlayerPawn 0))
  (if (and (< (.z (Transformation|GetActorLocation _returnvalue)) 1e+02) (Variables|Default|GetDown))
    (Utilities|FlowControl|DoOnce false
      (:Completed
        (Variables|Default|SetAlive? false)
        (Input|RemoveMappingContext (PlayerController|LocalPlayerSubsystems|GetEnhancedInputLocalPlayerSubsystem) "/Game/Starter/Assets/Inputs/IMC_GrannyControl.IMC_GrannyControl" "(bIgnoreAllPressedKeysUntilRelease=True,bForceImmediately=False,bNotifyUserSettings=False)")
        (bind _asgranny (Utilities|Casting|CastToGranny _returnvalue))
        (Components|Animation|PlayAnimation (Variables|/Script/Engine.Character|GetMesh _asgranny) "/Game/Starter/Assets/Granny/Animations/Standing_Death_Right_02.Standing_Death_Right_02" false)
        (Utilities|FlowControl|Delay 2.5)
        (Game|OpenLevel(byName) "StarterMap")))))

(event Input|KeyboardEvents|SpaceBar
  (params (Key :type Key%20Structure :default "None"))
  (bind _returnvalue (Game|Player|GetPlayerPawn 0))
  (bind _returnvalue_2 (PlayerController|LocalPlayerSubsystems|GetEnhancedInputLocalPlayerSubsystem))
  (:Pressed
    (if (Variables|Default|Gettransform?)
      (bind _returnvalue_3 (Game|SpawnActorfromClass "/Game/Starter/Blueprints/Granny.Granny_C" (Transformation|GetActorTransform _returnvalue) "Undefined" "MultiplyWithRoot" 0 0))
      (Actor|DestroyActor _returnvalue)
      (Pawn|Possess _returnvalue_3)
      (Input|RemoveMappingContext _returnvalue_2 "/Game/Starter/Assets/Inputs/IMC_AircraftControl.IMC_AircraftControl" "(bIgnoreAllPressedKeysUntilRelease=True,bForceImmediately=False,bNotifyUserSettings=False)")
      (Input|AddMappingContext _returnvalue_2 "/Game/Starter/Assets/Inputs/IMC_GrannyControl.IMC_GrannyControl" 0 "(bIgnoreAllPressedKeysUntilRelease=True,bForceImmediately=False,bNotifyUserSettings=False)")
      (Variables|Default|Settransform? false)
      (Variables|Default|SetDown true)
      (elif (< (.z (Transformation|GetActorLocation (Game|Player|GetPlayerPawn 0))) 1e+03)
        (Variables|Default|SetDown false)))))

(fn ConstructionScript)